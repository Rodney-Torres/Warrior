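; Enemy spawner actor that spawns queued enemy classes at its own transform.
; A looping timer spawns and dequeues the front entry, while adding to the queue also triggers an immediate spawn if no base enemy overlaps its Sphere.
; Each spawned enemy gets a destroyed-event binding, and an OnEnemyDefeated event forwards defeats to BP_BaseGameMode.
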(event Custom|TryToSpawn
  (CallFunction|SpawnEnemy))

(event Custom|OnEnemyDefeated
  (bind _asbp_base_game_mode (Utilities|Casting|CastToBP_BaseGameMode (Game|GetGameMode)))
  (Default|OnEnemyDefeated _asbp_base_game_mode))

(event EventBeginPlay
  (Utilities|Time|SetTimerbyEvent (delegate Custom|TryToSpawn) 2.0 true))

(fn ConstructionScript)

(fn SpawnEnemy
  (if (Utilities|Array|IsValidIndex (Variables|Default|GetEnemyQueue))
    (bind _returnvalue (Game|SpawnActorfromClass (Utilities|Array|Get(acopy) (Variables|Default|GetEnemyQueue)) (Transformation|GetActorTransform) "AdjustIfPossibleButAlwaysSpawn" "MultiplyWithRoot" 0 0))
    (EventDispatchers|BindEventtoOnDestroyed _returnvalue (EventDispatchers|CreateEvent :!event Custom|OnEnemyDefeated))
    (Utilities|Array|RemoveIndex (Variables|Default|GetEnemyQueue))
    (return true)
    (else
      (return false))))

(fn AddEnemytoQueue
  (params (EnemyClass :type BP%20Enemy%20Character%20Base%20Class%20Reference%20%28by%20ref%29))
  (Utilities|Array|Add (Variables|Default|GetEnemyQueue) EnemyClass)
  (if (not (Utilities|Array|IsValidIndex (Collision|GetOverlappingActors (Variables|Default|GetSphere) "/Game/EnemyCharacter/BP_EnemyCharacter_Base.BP_EnemyCharacter_Base_C" :!class /Script/Engine.PrimitiveComponent)))
    (CallFunction|SpawnEnemy)))