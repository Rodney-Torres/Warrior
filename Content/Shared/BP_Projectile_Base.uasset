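; Base projectile Blueprint that handles the audio and visual effects of a projectile's launch, flight and impact.
; BeginPlay plays a spawn sound, attaches a flight sound that stops when the attached component is destroyed, and spawns muzzle FX facing the actor's forward vector.
; OnSpawnProjectileHitFX plays the impact sound and FX at a given hit location.
; Each asset variable is validity-checked, and the graph contains no movement or damage logic.
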(event EventBeginPlay
  (Utilities|FlowControl|Sequence
    (:then_0
      ;[1 1 1] Play sound when the projectile is spawned
      (bind _projectilespawnsound (Variables|Default|GetProjectileSpawnSound)
        (:then
          (Audio|PlaySoundatLocation _projectilespawnsound (Transformation|GetActorLocation) "0, 0, 0" 1.0 1.0 0.0 0 0 0 0))
        (:else)))
    (:then_1
      ;[1 1 1] Play sound attached to a component and with the bool ticked we stop when the attached is destroyed
      (bind _projectileflysound (Variables|Default|GetProjectileFlySound)
        (:then
          (Audio|SpawnSoundAttached _projectileflysound (Variables|Transformation|GetRootComponent) "None" "0, 0, 0" "0, 0, 0" "KeepRelativeOffset" true 1.0 1.0 0.0 0 0))
        (:else)))
    (:then_2
      ;[1 1 1] Spawn muzzle FX system at location. Rotation matters here. Not sure what a muzzle FX is.
      (bind _projectilemuzzlefx (Variables|Default|GetProjectileMuzzleFX)
        (:then
          (Niagara|SpawnSystematLocation _projectilemuzzlefx (Transformation|GetActorLocation) (Math|Conversions|RotationFromXVector (Transformation|GetActorForwardVector))))
        (:else)))))

(event EventOnSpawnProjectileHitFX
  (params (HitLocation :type Vector%20%28by%20ref%29 :default "0, 0, 0"))
  ;[1 1 1] Play sound and spawn hit FX
  (Utilities|FlowControl|Sequence
    (:then_0
      ;[1 1 1] Play Sound
      (bind _projectileimpactsound (Variables|Default|GetProjectileImpactSound)
        (:then
          (Audio|PlaySoundatLocation _projectileimpactsound HitLocation "0, 0, 0" 1.0 1.0 0.0 0 0 0 0))
        (:else)))
    (:then_1
      ;[1 1 1] Spawn hit FX
      (bind _projectileimpactfx (Variables|Default|GetProjectileImpactFX)
        (:then
          (Niagara|SpawnSystematLocation _projectileimpactfx HitLocation))
        (:else)))))

(fn ConstructionScript)