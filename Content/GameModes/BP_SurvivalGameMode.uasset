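; Survival game mode Blueprint that shows on-screen wave announcements as the survival state changes.
; On BeginPlay it binds to the game mode state-changed delegate.
; The wait state creates a countdown widget timed by the spawn wait time, while the spawning state creates a widget showing the current wave number.
; Two helper functions create each widget, add it to the viewport and set its text.
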(event Custom|OnSurvivalGameModeStateChanged_Event
  (params (CurrentState :type EWarriorSurvivalGameModeState%20Enum :default "WaitSpawnNewWave"))
  (switch Utilities|FlowControl|Switch|SwitchonEWarriorSurvivalGameModeState CurrentState
    (:WaitSpawnNewWave
      ;[1 1 1] WaitSpawnNewWave -> Create widget and handle widget content
      (CallFunction|CreateWaveWidgetwithCountDown "New Wave Starting" (Variables|Default|GetSpawnNewWaveWaitTime)))
    (:SpawningNewWave
      ;[1 1 1] Displaying wave count widget
      (CallFunction|CreateWaveWidgetNoCountDown (Utilities|Text|FormatText "Wave {CurrentWaveCount}" (Variables|Default|GetCurrentWaveCount))))))

(event EventBeginPlay
  (EventDispatchers|AssignOnSurvivalGameModeStateChanged (delegate Custom|OnSurvivalGameModeStateChanged_Event)))

(event EventTick
  (params (DeltaSeconds :type Float%20%28single-precision%29)))

(fn ConstructionScript)

(fn CreateWaveWidgetwithCountDown
  (params (TextContentToDisplay :type Text) (InTotalCountDownTime :type Float%20%28double-precision%29))
  ;[1 1 1] Create widget -> Add to viewport -> Set text block content inside our widget class -> Start countdown
  (bind _returnvalue (UserInterface|CreateWidget "/Game/Widgets/GameModeWidgets/WBP_WaveTextWithCountDown.WBP_WaveTextWithCountDown_C"))
  (UserInterface|Viewport|AddtoViewport _returnvalue 0)
  ;[1 1 1] Set content, content is function input
  (Rendering|Components|TextRender|SetText (Variables|/Game/Widgets/GameModeWidgets/WBP_WaveTextWithCountDown.WBP_WaveTextWithCountDown_C|GetTextBlock_WaveText _returnvalue) TextContentToDisplay)
  ;[1 1 1] Function input we use another function input for specifying this
  (Default|StartCountDown _returnvalue InTotalCountDownTime))

(fn CreateWaveWidgetNoCountDown
  (params (TextContentToDisplay :type Text))
  (bind _returnvalue (UserInterface|CreateWidget "/Game/Widgets/GameModeWidgets/WBP_WaveTextNoCountDown.WBP_WaveTextNoCountDown_C"))
  (UserInterface|Viewport|AddtoViewport _returnvalue 0)
  ;[1 1 1] Setting text with function input
  (Rendering|Components|TextRender|SetText (Variables|/Game/Widgets/GameModeWidgets/WBP_WaveTextNoCountDown.WBP_WaveTextNoCountDown_C|GetTextBlock_WaveText _returnvalue) TextContentToDisplay))